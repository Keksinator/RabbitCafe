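; BP_NPC is a coffee shop customer that, after a random delay, asks for one of four coffees and reacts to what the player delivers.
; A sphere overlap outlines the NPC and enables ordering, which sets order flags and shows the recipe on screen.
; Delivery checks the player's held-coffee flags: success plays effects and restarts the cycle, failure shows an unhappy reaction.
; Status widgets and an indexed dialogue widget convey each state.
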(event OnComponentBeginOverlap(Sphere)
  (params (OverlappedComponent :type Primitive%20Component%20Object%20Reference) (OtherActor :type Actor%20Object%20Reference) (OtherComp :type Primitive%20Component%20Object%20Reference) (OtherBodyIndex :type Integer) (bFromSweep :type Boolean) (SweepResult :type Hit%20Result%20Structure%20%28by%20ref%29))
  ;[1 1 1 1 32] "E" To Interact Logic
  (bind _asbp_third_person_character (Utilities|Casting|CastToBP_Player OtherActor))
  (if (Variables|Default|GetWantsCoffee)
    (Rendering|SetVisibility (Variables|Default|GetInteractWidget) true false)
    (Variables|Default|SetPlayerInRangeForOrder true :!label _label)
    (Rendering|Material|SetOverlayMaterial (Variables|Character|GetMesh) "/Game/MaterialLibrary/M_Outline.M_Outline" :!class /Script/Engine.MeshComponent)
    (elif (Variables|/Game/Player/BP_Player.BP_Player_C|GetOrderAccepted _asbp_third_person_character)
      (goto _label))))

(event OnComponentEndOverlap(Sphere)
  (params (OverlappedComponent :type Primitive%20Component%20Object%20Reference) (OtherActor :type Actor%20Object%20Reference) (OtherComp :type Primitive%20Component%20Object%20Reference) (OtherBodyIndex :type Integer))
  ;[1 1 1 1 32] "E" To Interact Logic
  (if (Variables|Default|GetPlayerInRangeForOrder)
    (Utilities|Casting|CastToBP_Player OtherActor)
    (Rendering|SetVisibility (Variables|Default|GetInteractWidget) false false)
    (Variables|Default|SetPlayerInRangeForOrder false)
    (Rendering|Material|SetOverlayMaterial (Variables|Character|GetMesh) 0 :!class /Script/Engine.MeshComponent)))

(event Custom|OrderingRandomCoffee
  ;[1 1 1 1 32] Ordering Random Coffee/Order Being Taken
  (if (and (Variables|Default|GetPlayerInRangeForOrder) (Variables|Default|GetWantsCoffee))
    (bind _asbp_third_person_character (Utilities|Casting|CastToBP_Player (Game|GetPlayerCharacter 0)))
    (if (not (Variables|/Game/Player/BP_Player.BP_Player_C|GetOrderAccepted _asbp_third_person_character))
      (Variables|Default|SetCoffeeArrayNumber (Math|Random|RandomIntegerinRange 0 3))
      (bind _output_get (Variables|Default|SetCoffeeList (Variables|Default|GetCoffeeList)))
      (Variables|Default|SetCoffeeOrder (Utilities|Array|Get(acopy) _output_get (Variables|Default|GetCoffeeArrayNumber)))
      (if (== (Variables|Default|GetCoffeeArrayNumber) 0)
        (bind _output_get_2 (Variables|Default|SetWantsEspresso true))
        (Variables|/Game/Player/BP_Player.BP_Player_C|SetOrderAccepted _asbp_third_person_character true :!label _label)
        (Variables|Default|SetWantsCoffee false)
        (CallFunction|OrderTaken)
        (CallFunction|CoffeeType _output_get_2 (stale _output_get_3) (stale _output_get_4) (stale _output_get_5))
        (elif (== (Variables|Default|GetCoffeeArrayNumber) 1)
          (bind _output_get_3 (Variables|Default|SetWantsBlackCoffee true))
          (goto _label)
          (elif (== (Variables|Default|GetCoffeeArrayNumber) 2)
            (bind _output_get_4 (Variables|Default|SetWantsWhiteCoffee true))
            (goto _label)
            (elif (== (Variables|Default|GetCoffeeArrayNumber) 3)
              (bind _output_get_5 (Variables|Default|SetWantsLatte true))
              (goto _label))))))))

(event Custom|WantsToOrder
  ;[1 1 1 1 32] Wants To Order
  (Variables|Default|SetTalkIndex -1)
  (Utilities|FlowControl|Delay (Math|Random|RandomFloatinRange (Variables|Default|GetMinOrderWaitTime) (Variables|Default|GetMaxOrderWaitTime)))
  (Utilities|FlowControl|DoOnce false
    (:Completed
      (Rendering|SetVisibility (Variables|Default|GetWantsCoffeeWidget) true false)
      (Variables|Default|SetWantsCoffee true)
      (Variables|Default|SetInteractable true))))

(event Custom|OrderTaken
  ;[1 1 1 1 32] OrderTaken
  (Rendering|SetVisibility (Variables|Default|GetWantsCoffeeWidget) false false)
  (Rendering|SetVisibility (Variables|Default|GetWaitingCoffeeWidget) true false)
  (Audio|PlaySound2D "/Game/SFX/talking-nya-3-291989.talking-nya-3-291989" 1.0 1.0 0.0 0 0))

(event Custom|OrderDeliver
  (bind _mesh (Variables|Character|GetMesh))
  (bind _happywidget (Variables|Default|GetHappyWidget))
  (bind _unhappywidget (Variables|Default|GetUnhappyWidget))
  (bind _returnvalue (Transformation|GetWorldLocation _mesh))
  ;[1 1 1 1 32] OrderDelivery
  (if (and (Variables|Default|GetPlayerInRangeForOrder) (Math|Boolean|ORBoolean (Variables|Default|GetWantsEspresso) (Variables|Default|GetWantsBlackCoffee) (Variables|Default|GetWantsWhiteCoffee) (Variables|Default|GetWantsLatte)))
    (Variables|Default|SetBusy false)
    (bind _asbp_third_person_character (Utilities|Casting|CastToBP_Player (Game|GetPlayerCharacter 0)))
    (if (and (and (Variables|Default|GetWantsEspresso) (Variables|/Game/Player/BP_Player.BP_Player_C|GetHasEspresso _asbp_third_person_character)) (and (not (Variables|/Game/Player/BP_Player.BP_Player_C|GetHasBlackCoffee _asbp_third_person_character)) (not (Variables|/Game/Player/BP_Player.BP_Player_C|GetHasLatte _asbp_third_person_character))))
      (Variables|Default|SetDialogueOption "Thank you for my Espresso! :)")
      (Variables|Default|SetTalkIndex 0)
      (CallFunction|WantstoOrderReset :!label _label)
      (Utilities|FlowControl|Sequence
        (:then_0
          (Audio|PlaySound2D "/Game/SFX/happy-message-ping-351298.happy-message-ping-351298" 1.0 1.0 0.0 0 0))
        (:then_1
          (bind _asbp_third_person_character_2 (Utilities|Casting|CastToBP_Player (Game|GetPlayerCharacter 0)))
          (Default|Tracker _asbp_third_person_character_2)
          (Widget|SetVisibility (Variables|Default|GetCurrentUI) "Hidden")
          (Variables|/Game/Player/BP_Player.BP_Player_C|SetOrderAccepted _asbp_third_person_character false)
          (Variables|/Game/Player/BP_Player.BP_Player_C|SetHasCup _asbp_third_person_character false)
          (CallFunction|NotWantingCoffee)
          (Default|CoffeeBooleansReset _asbp_third_person_character)
          (bind _returnvalue_2 (Niagara|SpawnSystematLocation "/Game/VFX/NS_Stars.NS_Stars" (Math|Vector|MakeVector (.x _returnvalue) (.y _returnvalue) (+ (.z _returnvalue) 2e+02))))
          (Rendering|SetVisibility (Variables|Default|GetWaitingCoffeeWidget) false false)
          (Rendering|SetVisibility _happywidget true false)
          (Utilities|FlowControl|Delay 2.0)
          (Components|DestroyComponent _returnvalue_2)
          (Rendering|SetVisibility _happywidget false false)
          (CallFunction|WantstoOrder)
          (Variables|Default|SetTalkIndex -1)
          (Variables|Default|SetInteractable false)))
      (elif (and (Variables|Default|GetWantsBlackCoffee) (Variables|/Game/Player/BP_Player.BP_Player_C|GetHasBlackCoffee _asbp_third_person_character))
        (Variables|Default|SetDialogueOption "Thank you for my Black Coffee! :)")
        (Variables|Default|SetTalkIndex 0)
        (goto _label)
        (elif (and (Variables|Default|GetWantsWhiteCoffee) (Variables|/Game/Player/BP_Player.BP_Player_C|GetHasWhiteCoffee _asbp_third_person_character))
          (Variables|Default|SetDialogueOption "Thank you for my White Coffee! :)")
          (Variables|Default|SetTalkIndex 0)
          (goto _label)
          (elif (and (Variables|Default|GetWantsLatte) (Variables|/Game/Player/BP_Player.BP_Player_C|GetHasLatte _asbp_third_person_character))
            (Variables|Default|SetDialogueOption "Thank you for my Latte! :)")
            (Variables|Default|SetTalkIndex 0)
            (goto _label)
            (else
              (Variables|Default|SetDialogueOption "Where's my coffee? :(")
              (Variables|Default|SetTalkIndex 0)
              (Audio|PlaySound2D "/Game/SFX/training-program-incorrect2-88735.training-program-incorrect2-88735" 1.0 1.0 0.0 0 0)
              (Rendering|SetVisibility _unhappywidget true false)
              (Utilities|FlowControl|Delay 1.0)
              (Rendering|SetVisibility _unhappywidget false false))))))
    (else
      (Variables|Default|SetDialogueOption "(You already have an order!)")
      (Variables|Default|SetTalkIndex 0))))

(event Custom|WantsToOrderReset
  ;[1 1 1 1 32] Wants To Order
  (Utilities|FlowControl|DoOnce false) ; enters at Reset
)

(event Custom|NotWantingCoffee
  ;[1 1 1 1 32] OrderDelivery
  ;;[1 1 1] Unset Wanting Coffee
  (Variables|Default|SetWantsEspresso false)
  (Variables|Default|SetWantsLatte false)
  (Variables|Default|SetWantsBlackCoffee false)
  (Variables|Default|SetWantsWhiteCoffee false))

(event Custom|CoffeeType
  (params (Espresso :type Boolean) (Black :type Boolean) (White :type Boolean) (Latte :type Boolean))
  ;[1 1 1] CoffeeType
  (if Espresso
    (CallFunction|Current "Espresso: Cup + Espresso")
    (elif Black
      (CallFunction|Current "Black Coffee: Cup + Espresso + Water")
      (elif White
        (CallFunction|Current "White Coffee: Cup + Espresso + Milk + Water")
        (elif Latte
          (CallFunction|Current "Latte: Cup + Espresso + Milk"))))))

(event Custom|Current
  (params (CoffeeType :type String))
  ;[1 1 1] Current Coffee Tracker
  (bind _currentui (Variables|Default|GetCurrentUI)
    (:then
      (Widget|RemovefromParent _currentui))
    (:else
      _))
  (bind _returnvalue (UserInterface|CreateWidget "/Game/Blueprints/WB_Current.WB_Current_C" (Game|GetPlayerController 0)))
  (bind _output_get (Variables|Default|SetCurrentUI _returnvalue))
  (UserInterface|Viewport|AddtoViewport _output_get 0)
  (Rendering|Components|TextRender|SetText (Variables|/Game/Blueprints/WB_Current.WB_Current_C|GetTalkText (Variables|Default|GetCurrentUI)) (Utilities|Text|ToText(String) CoffeeType))
  (Widget|SetVisibility (Variables|Default|GetCurrentUI) "Visible"))

(event EventBeginPlay
  ;[1 1 1 1 32] BeginPlayEvents
  (Rendering|SetVisibility (Variables|Default|GetInteractWidget) false false)
  (Rendering|SetVisibility (Variables|Default|GetWantsCoffeeWidget) false false)
  (Rendering|SetVisibility (Variables|Default|GetWaitingCoffeeWidget) false false)
  (Rendering|SetVisibility (Variables|Default|GetHappyWidget) false false)
  (Rendering|SetVisibility (Variables|Default|GetUnhappyWidget) false false)
  (CallFunction|WantstoOrder))

(event EventTalk
  ;[1 1 1] Dialogue
  (if (Variables|Default|GetInteractable)
    (Variables|Default|SetDialogue (Utilities|Array|MakeArray (Variables|Default|GetCoffeeOrder) (Variables|Default|GetDialogueOption)))
    (Math|Integer|IncrementInt (Variables|Default|GetTalkIndex)
      (:%20%20
        (if (<= (Variables|Default|GetTalkIndex) (Utilities|Array|Length (Variables|Default|GetDialogue)))
          (bind _ui (Variables|Default|GetUI)
            (:then
              (Widget|RemovefromParent _ui))
            (:else
              _))
          (bind _returnvalue (UserInterface|CreateWidget "/Game/Blueprints/WB_Dialogue.WB_Dialogue_C" (Game|GetPlayerController 0)))
          (bind _output_get (Variables|Default|SetUI _returnvalue))
          (UserInterface|Viewport|AddtoViewport _output_get 0)
          (if (Utilities|Enum|Equal(Enum) (Utilities|Array|Get(acopy) (Variables|Default|GetDialogue) (Variables|Default|GetTalkIndex)) "(You already have an order!)")
            (Rendering|Components|TextRender|SetText (Variables|/Game/Blueprints/WB_Dialogue.WB_Dialogue_C|GetTalkText (Variables|Default|GetUI)) "(You already have an order!)")
            (Widget|SetVisibility (Variables|Default|GetUI) "Visible" :!label _label)
            (Utilities|FlowControl|Delay 2.0)
            (elif (Utilities|Enum|Equal(Enum) (Utilities|Array|Get(acopy) (Variables|Default|GetDialogue) (Variables|Default|GetTalkIndex)) "")
              _
              (else
                (Rendering|Components|TextRender|SetText (Variables|/Game/Blueprints/WB_Dialogue.WB_Dialogue_C|GetTalkText (Variables|Default|GetUI)) (Utilities|Text|ToText(String) (Utilities|String|Append "\"" (Utilities|Array|Get(acopy) (Variables|Default|GetDialogue) (Variables|Default|GetTalkIndex)) "\"")))
                (goto _label))))
          (Widget|SetVisibility (Variables|Default|GetUI) "Hidden"))))))

(fn ConstructionScript)